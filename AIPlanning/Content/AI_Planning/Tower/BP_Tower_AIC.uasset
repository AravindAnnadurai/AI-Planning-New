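; BP_Tower_AIC is the AI controller for BP_Tower, tracking the actors the tower can currently see as potential targets.
; On possessing a BP_Tower, it caches the pawn and runs BT_Tower.
; Sight perception updates add sensed actors to a unique target list and remove them when sight is lost.
; ChooseTargetActor returns a random actor from that list, or nothing when it is empty.
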(event OnTargetPerceptionUpdated(AIPerception)
  (params (Actor :type Actor%20Object%20Reference) (Stimulus :type AI%20Stimulus%20Structure))
  (bind _returnvalue (Class|AIPerceptionSystem|GetSenseClassforStimulus Stimulus))
  (if (== _returnvalue "/Script/AIModule.AISense_Sight")
    (if (.bSuccessfullySensed (Utilities|Struct|BreakAIStimulus Stimulus))
      (Utilities|Array|AddUnique (Variables|Default|GetAllTargetActors) Actor)
      (else
        (CallFunction|RemoveTargetActor Actor)))))

(event EventPossess
  (params (PossessedPawn :type Pawn%20Object%20Reference))
  (bind _asbp_tower (Utilities|Casting|CastToBP_Tower PossessedPawn))
  (Variables|Default|SetAs%20BP%20Tower _asbp_tower)
  (AI|RunBehaviorTree "/Game/AI_Planning/Tower/BT_Tower.BT_Tower"))

(fn ConstructionScript)

(fn RemoveTargetActor
  (params (TargetActor :type Actor%20Object%20Reference%20%28by%20ref%29))
  (Utilities|Array|RemoveItem (Variables|Default|GetAllTargetActors) TargetActor))

(fn ChooseTargetActor
  (if (Utilities|Array|IsNotEmpty (Variables|Default|GetAllTargetActors))
    (return (.OutItem (Utilities|Array|Random (Variables|Default|GetAllTargetActors))))
    (else
      (return 0))))